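; BP_SpaceShip is a spaceship Blueprint whose only working logic switches between cockpit and external camera views.
; The ToggleCameraView input drives a FlipFlop that activates one camera and deactivates the other on alternate presses.
; The Roll axis event is empty, and leftover nodes involving ThrustStrength and RollStrength are disconnected, so the graph implements no flight movement.
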(event `InputAxis|Roll`
  (params (AxisValue :type "Float (single-precision)")))

(event `InputAction|ToggleCameraView`
  (params (Key :type "Key Structure" :default "AnyKey"))
  (bind _externalcamera (`self.ExternalCamera`))
  (bind _cockpitcamera (`self.CockpitCamera`))
  ;[1 1 1] Camera Switcher
  (:`Pressed`
    (`/Engine/EditorBlueprintResources/StandardMacros.FlipFlop`
      (:`A`
        (`ActorComponent.Activate` _cockpitcamera false)
        (`ActorComponent.Deactivate` _externalcamera))
      (:`B`
        (`ActorComponent.Deactivate` _cockpitcamera)
        (`ActorComponent.Activate` _externalcamera false)))))

(fn `UserConstructionScript`)