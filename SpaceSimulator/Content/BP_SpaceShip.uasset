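; Player-controlled spaceship Blueprint that flies by applying physics forces from input axes.
; Pitch, roll and yaw each drive a pair of thruster components, scaled by a shared strength variable and deactivated at zero input.
; Engine thrust adds an impulse to the static mesh along the root arrow's forward vector, without delta-time scaling.
; A camera input flip-flops between cockpit and third-person views.
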(event `InputAction|ToogleCamera`
  (params (Key :type "Key Structure" :default "AnyKey"))
  (bind _cockpitcamera (`self.CockpitCamera`))
  (bind _thirdpersoncamera (`self.ThirdPersonCamera`))
  ;[1 1 1] Camera Views
  (:`Pressed`
    (`/Engine/EditorBlueprintResources/StandardMacros.FlipFlop`
      (:`A`
        (`ActorComponent.Deactivate` _thirdpersoncamera)
        (`ActorComponent.Activate` _cockpitcamera false))
      (:`B`
        (`ActorComponent.Deactivate` _cockpitcamera)
        (`ActorComponent.Activate` _thirdpersoncamera false)))))

(event `InputAxis|Pitch`
  (params (AxisValue :type "Float (single-precision)"))
  (bind _nosepitchthrust (`self.NosePitchThrust`))
  (bind _returnvalue (* AxisValue (`self.RollStringth`)))
  ;[1 1 1] Pitch
  (if (!= AxisValue 0.0)
    (set `PhysicsThrusterComponent.ThrustStrength` _returnvalue _nosepitchthrust)
    (set `PhysicsThrusterComponent.ThrustStrength` _returnvalue (`self.TaillPitchThrust`))
    (`ActorComponent.Activate` _nosepitchthrust false)
    (`ActorComponent.Activate` (`self.TaillPitchThrust`) false)
    (else
      (`ActorComponent.Deactivate` _nosepitchthrust)
      (`ActorComponent.Deactivate` (`self.TaillPitchThrust`)))))

(event `InputAxis|Roll`
  (params (AxisValue :type "Float (single-precision)"))
  (bind _leftwingrollthrust (`self.LeftWingRollThrust`))
  (bind _returnvalue (* AxisValue (`self.RollStringth`)))
  ;[1 1 1] Roll
  (if (!= AxisValue 0.0)
    (set `PhysicsThrusterComponent.ThrustStrength` _returnvalue _leftwingrollthrust)
    (set `PhysicsThrusterComponent.ThrustStrength` _returnvalue (`self.RightWingRollThrust`))
    (`ActorComponent.Activate` _leftwingrollthrust false)
    (`ActorComponent.Activate` (`self.RightWingRollThrust`) false)
    (else
      (`ActorComponent.Deactivate` _leftwingrollthrust)
      (`ActorComponent.Deactivate` (`self.RightWingRollThrust`)))))

(event `InputAxis|Yaw`
  (params (AxisValue :type "Float (single-precision)"))
  (bind _noseyawthrust (`self.NoseYawThrust`))
  (bind _returnvalue (* AxisValue (`self.RollStringth`)))
  ;[1 1 1] Yaw
  (if (!= AxisValue 0.0)
    (set `PhysicsThrusterComponent.ThrustStrength` _returnvalue _noseyawthrust)
    (set `PhysicsThrusterComponent.ThrustStrength` _returnvalue (`self.TailYawThrust`))
    (`ActorComponent.Activate` _noseyawthrust false)
    (`ActorComponent.Activate` (`self.TailYawThrust`) false)
    (else
      (`ActorComponent.Deactivate` _noseyawthrust)
      (`ActorComponent.Deactivate` (`self.TailYawThrust`)))))

(event `InputAxis|EngineThrust`
  (params (AxisValue :type "Float (single-precision)"))
  (`PrimitiveComponent.AddImpulse` (`self.StaticMesh`) (* (`KismetMathLibrary.GetForwardVector` (`SceneComponent.K2_GetComponentRotation` (`self.RootDirectionArrow`))) (* AxisValue (`self.EnginePower`))) "None" false))

(fn `UserConstructionScript`)